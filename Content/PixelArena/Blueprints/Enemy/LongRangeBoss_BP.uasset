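; Long-range boss enemy for a 2D flipbook arena that cycles through five fixed teleport points.
; After BeginPlay, BossMovement re-triggers itself every few seconds, looping the cast animation and setting a timer for Teleporting.
; Casting steps a wrapping counter that GetPosition maps to coordinates; Teleporting calls teleport and appear flipbooks back to back, without waiting.
; State events are empty stubs, and casting spawns no attack.
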(event Custom|BossMovement
  (CallFunction|Casting)
  (Utilities|Time|SetTimerbyFunctionName 0 "Teleporting" 5.0)
  (Utilities|FlowControl|Delay 5.2)
  (CallFunction|BossMovement))

(event EventAttackState
  (params (AttackTime :type Float%20%28single-precision%29) (AttackDown :type Boolean)))

(event EventAbilityState
  (params (AbilityTime :type Float%20%28single-precision%29) (AbilityDown :type Boolean)))

(event EventWalkingState)

(event EventAnimationFinished)

(event EventBeginPlay
  (Utilities|FlowControl|Delay 1.0)
  (CallFunction|BossMovement))

(event EventIdleState)

(fn ConstructionScript)

(fn Casting
  (bind _output_get (Variables|Default|Setintvalue (- (Variables|Default|Getintvalue) 1)))
  (if (== (Variables|Default|Getintvalue) 0)
    (Variables|Default|Setintvalue 5))
  (Development|PrintString (Utilities|String|ToString(Integer) _output_get))
  (Class|ArenaCharacter|PlayFlipbook "/Game/PixelArena/Flipbooks/Boss/LongRangeBossCast.LongRangeBossCast" true))

(fn Teleporting
  (Class|ArenaCharacter|PlayFlipbook "/Game/PixelArena/Flipbooks/Boss/LongRangeBossTeleport.LongRangeBossTeleport" false)
  (CallFunction|GetPosition)
  (Transformation|Teleport (Math|Vector|MakeVector (Variables|Default|GetPos_X) 0.0 (Variables|Default|GetPos_Z)) "0, 0, 0")
  (Class|ArenaCharacter|PlayFlipbook "/Game/PixelArena/Flipbooks/Boss/LongRangeBossAppear.LongRangeBossAppear" false))

(fn GetPosition
  (if (== (Variables|Default|Getintvalue) 4)
    (Variables|Default|SetPos_X -2423.27832)
    (Variables|Default|SetPos_Z 3452.393555)
    (elif (== (Variables|Default|Getintvalue) 3)
      (Variables|Default|SetPos_X -2417.0)
      (Variables|Default|SetPos_Z 2974.0)
      (elif (== (Variables|Default|Getintvalue) 2)
        (Variables|Default|SetPos_X -1594.0)
        (Variables|Default|SetPos_Z 2974.0)
        (elif (== (Variables|Default|Getintvalue) 1)
          (Variables|Default|SetPos_X -1594.0)
          (Variables|Default|SetPos_Z 3414.0)
          (elif (== (Variables|Default|Getintvalue) 5)
            (Variables|Default|SetPos_X -2008.0)
            (Variables|Default|SetPos_Z 3302.870361)))))))