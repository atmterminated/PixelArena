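; Shield-wielding character Blueprint for PixelArena that supplies the attack and shield animations on top of its parent class.
; Attack and ability state events play one-shot flipbooks chosen from per-state maps by facing direction.
; The shield ability finishes when the ability input is no longer down, while an attack finishes when its animation completes during the Attacking state.
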(event EventAttackState
  (params (AttackTime :type Float%20%28single-precision%29) (AttackDown :type Boolean))
  ;[1 0.1925 0.2822] Attack State
  (Class|ArenaCharacter|PlayFlipbook (Utilities|GetFlipbookfromDirection (Variables|Default|GetAttackAnimations) (Variables|Default|GetFacing)) false))

(event EventAnimationFinished
  ;[0.2754 0.2314 1] Animation FInished
  (switch Utilities|FlowControl|Switch|SwitchonCharacterState (Variables|Default|GetCharacterState)
    (:Attacking
      (Class|ArenaCharacter|FinishAttack))))

(event EventAbilityState
  (params (AbilityTime :type Float%20%28single-precision%29) (AbilityDown :type Boolean))
  ;[0.4509 1 0.394] Shield State
  (if AbilityDown
    (Class|ArenaCharacter|PlayFlipbook (Utilities|GetFlipbookfromDirection (Variables|Default|GetShieldAnimations) (Variables|Default|GetFacing)) false)
    (else
      (Class|ArenaCharacter|FinishAbility))))

(fn ConstructionScript
  (|CallParentFunction))