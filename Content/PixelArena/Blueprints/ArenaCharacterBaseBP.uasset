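; Base Blueprint for arena characters in PixelArena, providing per-state events and access to the pause menu.
; The walking state event calls Move, while the idle, attack, ability and animation-finished events are empty.
; Pressing Escape creates the UIPause widget if none is valid, reuses it otherwise, then shows the cursor, switches to UI-only input and pauses the game.
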(event EventAttackState
  (params (AttackTime :type Float%20%28single-precision%29) (AttackDown :type Boolean)))

(event EventAbilityState
  (params (AbilityTime :type Float%20%28single-precision%29) (AbilityDown :type Boolean)))

(event EventAnimationFinished)

(event EventIdleState)

(event EventWalkingState
  (Class|ArenaCharacter|Move))

(event Input|KeyboardEvents|Escape
  (params (Key :type Key%20Structure :default "None"))
  (bind _returnvalue (Game|GetPlayerController 0))
  (:Pressed
    (Utilities|IsValid (Variables|Default|GetPause%20Menu)
      (:Is%20Valid
        _)
      (:Is%20Not%20Valid
        (bind _returnvalue_2 (UserInterface|CreateWidget "/Game/PixelArena/UI/UIPause.UIPause_C"))
        (Variables|Default|SetPause%20Menu _returnvalue_2)))
    (Variables|/Script/Engine.PlayerController|SetbShowMouseCursor _returnvalue true)
    (Input|SetInputModeUIOnly _returnvalue (Variables|Default|GetPause%20Menu) "DoNotLock")
    (UserInterface|Viewport|AddtoViewport (Variables|Default|GetPause%20Menu) 0)
    (Game|SetGamePaused true)))

(fn ConstructionScript)